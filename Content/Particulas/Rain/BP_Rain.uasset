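; BP_Rain is a rain effect actor whose wind can be steered from the keyboard.
; On BeginPlay it enables input for player controller 0.
; Each arrow key press adds a fixed horizontal step to an accumulated wind vector along X or Y, then pushes it to the FXRain particle component's WindForce vector parameter.
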(event EventBeginPlay
  (Input|EnableInput (Game|GetPlayerController 0)))

(event Collision|EventActorBeginOverlap
  (params (OtherActor :type Actor%20Object%20Reference)))

(event EventTick
  (params (DeltaSeconds :type Float%20%28single-precision%29)))

(event Input|KeyboardEvents|Down
  (params (Key :type Key%20Structure :default "None"))
  (:Pressed
    (Variables|Default|SetWindFoece (+ (Variables|Default|GetWindFoece) "0.000000,250.000000,0.000000"))
    (Effects|Components|ParticleSystem|SetVectorParameter (Variables|Default|GetFX_Rain) "WindForce" (Variables|Default|GetWindFoece))))

(event Input|KeyboardEvents|Right
  (params (Key :type Key%20Structure :default "None"))
  (:Pressed
    (Variables|Default|SetWindFoece (+ (Variables|Default|GetWindFoece) "250.000000,0.000000,0.000000"))
    (Effects|Components|ParticleSystem|SetVectorParameter (Variables|Default|GetFX_Rain) "WindForce" (Variables|Default|GetWindFoece))))

(event Input|KeyboardEvents|Up
  (params (Key :type Key%20Structure :default "None"))
  (:Pressed
    (Variables|Default|SetWindFoece (+ (Variables|Default|GetWindFoece) "0.000000,-250.000000,0.000000"))
    (Effects|Components|ParticleSystem|SetVectorParameter (Variables|Default|GetFX_Rain) "WindForce" (Variables|Default|GetWindFoece))))

(event Input|KeyboardEvents|Left
  (params (Key :type Key%20Structure :default "None"))
  (:Pressed
    (Variables|Default|SetWindFoece (+ (Variables|Default|GetWindFoece) "-250.000000,0.000000,0.000000"))
    (Effects|Components|ParticleSystem|SetVectorParameter (Variables|Default|GetFX_Rain) "WindForce" (Variables|Default|GetWindFoece))))

(fn ConstructionScript)