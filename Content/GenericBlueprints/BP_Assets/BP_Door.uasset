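; Interactable door actor that swings a pivot between closed and an OpenAngle yaw.
; BeginPlay sets the timeline length to AnimationDuration and its start time from IsOpen.
; Interact toggles IsOpen and calls SetOpen, which plays or reverses OpenCloseTimeline through its component reference.
; The timeline's Update derives DoorPivot's relative yaw from normalized playback position rather than a track output.
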(event EventBeginPlay
  (bind _openclosetimeline (Variables|Default|GetOpenCloseTimeline))
  (Components|Timeline|SetTimelineLength (Variables|Default|GetOpenCloseTimeline) (Variables|Default|GetAnimationDuration))
  (if (Variables|Default|GetIsOpen)
    (Components|Timeline|SetNewTime _openclosetimeline (Components|Timeline|GetTimelineLength _openclosetimeline))
    (else
      (Components|Timeline|SetNewTime _openclosetimeline 0.0))))

(event Collision|EventActorBeginOverlap
  (params (OtherActor :type Actor%20Object%20Reference)))

(event EventTick
  (params (DeltaSeconds :type Float%20%28single-precision%29)))

(event EventInteract
  (bind _output_get (Variables|Default|SetIsOpen (not (Variables|Default|GetIsOpen))))
  (CallFunction|SetOpen _output_get))

(fn ConstructionScript)

(fn SetOpen
  (params (SetOpen :type Boolean))
  (bind _openclosetimeline (Variables|Default|GetOpenCloseTimeline))
  (if SetOpen
    (Audio|Components|Audio|Play _openclosetimeline)
    (else
      (Utilities|String|Reverse _openclosetimeline))))