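; Game Instance Blueprint that owns the game's persistent save data.
; On Init it loads the save slot and caches the result as a BP_Global_SG SaveGame object.
; If the load does not yield a valid object, it creates a new one and immediately writes it through SaveData, which saves the cached object to the same slot.
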(event EventInit
  (CallFunction|LoadSaveData))

(fn SaveData
  (SaveGame|SaveGametoSlot (Variables|Default|GetSaveGame) (Variables|Default|GetSaveDataSlotName)))

(fn LoadSaveData
  (bind _returnvalue (SaveGame|LoadGamefromSlot (Variables|Default|GetSaveDataSlotName)))
  (bind _asbp_global_sg (Utilities|Casting|CastToBP_Global_SG _returnvalue)
    (:then
      (Development|PrintString "ExisteSaveData")
      (Variables|Default|SetSaveGame _asbp_global_sg))
    (:CastFailed
      (Development|PrintString "No Existe Save Data")
      (bind _returnvalue_2 (SaveGame|CreateSaveGameObject "/Game/GenericBlueprints/BP_Setup/BP_Global_SG.BP_Global_SG_C"))
      (Variables|Default|SetSaveGame _returnvalue_2)
      (CallFunction|SaveData))))